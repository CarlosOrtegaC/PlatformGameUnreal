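; Enemy bullet actor that damages the third-person player character on overlap.
; Tick moves it along its forward vector at Speed, scaled by delta time, without sweeping.
; Overlapping a BP_ThirdPersonCharacter calls that character's damage event directly with a fixed amount and destroys the bullet, while other actors are ignored.
; A timer started on BeginPlay destroys the bullet after a short lifetime.
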(event Custom|Destroy
  (Actor|DestroyActor))

(event EventBeginPlay
  (Utilities|Time|SetTimerbyEvent (delegate Custom|Destroy) 3.0))

(event EventTick
  (params (DeltaSeconds :type Float%20%28single-precision%29))
  (Transformation|SetActorLocation (+ (Transformation|GetActorLocation) (* (* DeltaSeconds (Variables|Default|GetSpeed)) (Transformation|GetActorForwardVector))) false false))

(event Collision|EventActorBeginOverlap
  (params (OtherActor :type Actor%20Object%20Reference))
  (bind _asbp_third_person_character (Utilities|Casting|CastToBP_ThirdPersonCharacter OtherActor))
  (Default|OnTakeAnyDamageEvent0 _asbp_third_person_character 0 5.0)
  (Actor|DestroyActor))

(fn ConstructionScript)